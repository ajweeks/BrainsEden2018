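; Character health Blueprint for a two-sided Hot/Ice game, tracking damage and reporting death to the game instance.
; Health is signed: Icey rises from -100 to die at +100, the other side mirrors it; BeginPlay currently hard-codes non-Icey.
; Tick applies DPS while on enemy territory.
; On death it passes player controller 0's ID, regardless of owner, to GI_HotAsIce's PlayerWinAndChecks.
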(event `self.ReceiveBeginPlay`
  (bind _output_get (set `self.IsIcey` false))
  (if _output_get
    (set `self.Health` -100.0)
    (else
      (set `self.Health` 100.0))))

(event `OnEnemyTerritory`
  (params (`Delta Seconds` :type "Float (double-precision)"))
  ;[1 1 1] Do damage on EnemyTerritory
  (if (`self.IsOnEnemyTerritory`)
    (`self.TakeDamageAndCheck` (* `Delta Seconds` (`self.DPSOnEnemyTerritory`)))))

(event `TakeDamageAndCheck`
  (params (Damage :type "Float (double-precision)"))
  ;[1 1 1] Take Damage and check for win
  (`self.TakeDamage` Damage)
  (bind _death (`self.IsDeath`))
  (if _death
    (bind _asgi_hot_as_ice (cast `/Game/Blueprints/GameMode/GI_HotAsIce` (`GameplayStatics.GetGameInstance`)))
    (bind _returnvalue (`GameplayStatics.GetPlayerControllerID` (`GameplayStatics.GetPlayerController` 0)))
    (`/Game/Blueprints/GameMode/GI_HotAsIce.PlayerWinAndChecks` _asgi_hot_as_ice _returnvalue)))

(event `self.ReceiveTick`
  (params (DeltaSeconds :type "Float (single-precision)"))
  ;[1 1 1] Tick
  (`|ExecutionSequence`
    (:`then_0`
      (`self.OnEnemyTerritory` DeltaSeconds))))

(fn `IsDeath`
  (returns (death :type Boolean))
  (if (`self.IsIcey`)
    (if (>= (`self.Health`) 100.0)
      _
      (else
        (return false)))
    (elif (<= (`self.Health`) -100.0)
      _
      (else
        (return false))))
  (return true))

(fn `TakeDamage`
  (params (damage :type "Float (double-precision)"))
  (returns (health :type "Float (double-precision)"))
  ;[1 1 1] gets damage amount in(should be +)/ returns current health
  (if (`self.IsIcey`)
    (bind _output_get (set `self.Health` (+ (`self.Health`) damage)))
    (return _output_get)
    (else
      (bind _output_get_2 (set `self.Health` (- (`self.Health`) damage)))
      (return _output_get_2))))