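; Player character for two local players, with movement and slide input filtered by Index; Player 1's horizontal axis is unwired.
; Holding slide changes the movement multiplier, while exceeding the time limit only prints a warning.
; Holding spray runs a debug-drawn sphere overlap each tick, calling Cooldown on BP_Tile actors with positive damage for Ice, negative for Fire.
; Spraying and the debug Ice/Fire swap ignore Index.
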(event `self.ReceiveTick`
  (params (DeltaSeconds :type "Float (single-precision)"))
  (`|ExecutionSequence`
    (:`then_0`
      (if (`self.Sliding`)
        (bind _output_get (set `self.SecondsSliding` (+ (`self.SecondsSliding`) DeltaSeconds)))
        (if (> _output_get (`self.MaxSecondsSliding`))
          (`KismetSystemLibrary.PrintString` "Slid too long!"))))
    (:`then_1`
      (if (`self.IsSpraying`)
        (`self.Spraying`)))))

(event `InputAxis|Player0_MoveHorizontal`
  (params (AxisValue :type "Float (single-precision)"))
  (if (== (`self.Index`) 0)
    (`self.AddMovementInput` (`self.GetActorRightVector`) (* AxisValue (`self.CurrentMoveMultiplier`)))))

(event `InputAxis|Player0_MoveVertical`
  (params (AxisValue :type "Float (single-precision)"))
  (if (== (`self.Index`) 0)
    (`self.AddMovementInput` (`self.GetActorForwardVector`) (* AxisValue (`self.CurrentMoveMultiplier`)))))

(event `InputAxis|Player1_MoveHoriztonal`
  (params (AxisValue :type "Float (single-precision)")))

(event `InputAxis|Player1_MoveVertical`
  (params (AxisValue :type "Float (single-precision)"))
  (if (== (`self.Index`) 1)
    (`self.AddMovementInput` (`self.GetActorForwardVector`) (* AxisValue (`self.CurrentMoveMultiplier`)))))

(event `InputAction|Player0_Slide`
  (params (Key :type "Key Structure"))
  (:`Pressed`
    (if (and (== (`self.Index`) 0) (not (`self.Sliding`)))
      (set `self.Sliding` true)
      (set `self.SecondsSliding` 0.0)
      (set `self.CurrentMoveMultiplier` (`self.SlidingMoveSpeedMultiplier`))))
  (:`Released`
    (if (and (== (`self.Index`) 0) (`self.Sliding`))
      (set `self.Sliding` false)
      (set `self.CurrentMoveMultiplier` 1.0))))

(event `InputAction|Player1_Slide`
  (params (Key :type "Key Structure"))
  (:`Pressed`
    (if (and (== (`self.Index`) 1) (not (`self.Sliding`)))
      (set `self.Sliding` true)
      (set `self.SecondsSliding` 0.0)
      (set `self.CurrentMoveMultiplier` (`self.SlidingMoveSpeedMultiplier`))))
  (:`Released`
    (if (and (== (`self.Index`) 1) (`self.Sliding`))
      (set `self.Sliding` false)
      (set `self.CurrentMoveMultiplier` 1.0))))

(event `InputAction|Spraying`
  (params (Key :type "Key Structure"))
  (:`Pressed`
    (set `self.IsSpraying` true))
  (:`Released`
    (set `self.IsSpraying` false)))

(event `Spraying`
  (`KismetSystemLibrary.DrawDebugSphere` (`SceneComponent.K2_GetComponentLocation` (`self.SpraySphereOverlapPosition`)) (`self.SprayingSphereSize`) 12 (struct :`R` 1.0 :`G` 0.007851 :`A` 1.0) 0.0 1.0)
  (bind _outactors (`KismetSystemLibrary.SphereOverlapActors` (`SceneComponent.K2_GetComponentLocation` (`self.SpraySphereOverlapPosition`)) (`self.SprayingSphereSize`) (`|MakeArray` "ObjectTypeQuery1" :!type "EObjectTypeQuery Enum") "/Game/Blueprints/Tiles/BP_Tile.BP_Tile_C"))
  (for _array_element _outactors
    (switch `/Game/Blueprints/Character/Types` (`self.Type`)
      (:`NewEnumerator0`
        (bind _asbp_tile (cast `/Game/Blueprints/Tiles/BP_Tile` _array_element))
        (`/Game/Blueprints/Tiles/BP_Tile.Cooldown` _asbp_tile (`self.SprayDamage`)))
      (:`NewEnumerator1`
        (bind _asbp_tile_2 (cast `/Game/Blueprints/Tiles/BP_Tile` _array_element))
        (`/Game/Blueprints/Tiles/BP_Tile.Cooldown` _asbp_tile_2 (* (`self.SprayDamage`) -1.0))))))

(event `InputAction|TEMPTypeSwapping`
  (params (Key :type "Key Structure"))
  ;[1 0 0.05494] DEBUG
  (:`Pressed`
    (switch `/Game/Blueprints/Character/Types` (`self.Type`)
      (:`NewEnumerator0`
        (set `self.Type` "NewEnumerator1"))
      (:`NewEnumerator1`
        (set `self.Type` "NewEnumerator0")))))

(fn `UserConstructionScript`)