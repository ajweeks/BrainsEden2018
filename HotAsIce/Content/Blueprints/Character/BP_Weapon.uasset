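; Charge-and-release weapon for Player_BP that launches BP_Projectile fireballs and adds heat to the player on each shot.
; Fire toggles the input state; holding builds charge, and release (with no live fireball) or max charge spawns the projectile.
; Charge lerps the landing point along the barrel's forward, previewed by a BP_Marker parked far away when idle or overheated.
; Shots set a Recharging lock, cleared by delayed Recharge; unreliability logic is unwired.
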(event `self.ReceiveBeginPlay`
  ;[1 1 1] BEGIN PLAY
  ;;[1 1 1] Get reference to player
  (bind _asplayer_bp (cast `/Game/Blueprints/Character/Player_BP` (`self.GetOwner`)))
  (set `self.OwnerReference` _asplayer_bp)
  (bind _returnvalue (`|SpawnActorFromClass` "/Game/Blueprints/Character/BP_Marker.BP_Marker_C" (`KismetMathLibrary.MakeTransform` (1000000.0 10000.0 10000.0)) "AlwaysSpawn" "OverrideRootScale" null null))
  (set `self.Marker` _returnvalue))

(event `Fire`
  (`|ExecutionSequence`
    (:`then_0`
      ;[1 1 1] Player just released button
      (`/Engine/EditorBlueprintResources/StandardMacros.IsValid` (`self.FireballRef`)
        (:`Is Not Valid`
          (if (`self.IsInputDown`)
            (if (not (`self.Recharging`))
              (`self.CreateProjectile`))))))
    (:`then_1`
      ;[1 1 1] Toggle the bool
      (set `self.IsInputDown` (not (`self.IsInputDown`))))))

(event `CreateProjectile`
  ;[1 1 1] Create projectile
  (if (not (`/Game/Blueprints/Character/Player_BP.IsOverheated` (`self.OwnerReference`)))
    (`|ExecutionSequence`
      (:`then_0`
        (bind _returnvalue (`|SpawnActorFromClass` "/Game/Blueprints/Projectiles/BP_Projectile.BP_Projectile_C" (`KismetMathLibrary.MakeTransform` (0.0 0.0 0.0)) "AlwaysSpawn" "OverrideRootScale" null null))
        (bind _output_get (set `self.FireballRef` _returnvalue))
        (`Actor.SetOwner` _output_get (`self.OwnerReference`))
        (set `/Game/Blueprints/Projectiles/BP_Projectile.BeginPoint` (`SceneComponent.K2_GetComponentLocation` (`/Game/Blueprints/Character/Player_BP.GunBarrel` (`self.OwnerReference`))) (`self.FireballRef`))
        (set `/Game/Blueprints/Projectiles/BP_Projectile.EndPoint` (`self.CalculateLandingPosition`) (`self.FireballRef`))
        (`/Game/Blueprints/Character/Player_BP.AddHeat` (`self.OwnerReference`) (`self.GunHeatAddition`)))
      (:`then_1`
        (set `self.ChargeTimer` 0.0)
        (set `self.Recharging` true)))))

(event `self.ReceiveTick`
  (params (DeltaSeconds :type "Float (single-precision)"))
  ;[1 1 1] TICK
  (if (`/Game/Blueprints/Character/Player_BP.IsOverheated` (`self.OwnerReference`))
    (`Actor.K2_SetActorLocation` (`self.Marker`) (10000.0 10000.0 10000.0) false true)
    (else
      (`|ExecutionSequence`
        (:`then_0`
          ;;[1 1 1] Handle Input
          (if (`self.IsInputDown`)
            (if (not (`self.Recharging`))
              (set `self.ChargeTimer` (+ (`self.ChargeTimer`) (`GameplayStatics.GetWorldDeltaSeconds`)))
              (if (>= (`self.ChargeTimer`) (`self.MaxChargeTime`))
                (`self.CreateProjectile`)))))
        (:`then_2`
          (if (>= (`self.ChargeTimer`) 0.005)
            (`Actor.K2_SetActorLocation` (`self.Marker`) (`self.CalculateLandingPosition`) false true)
            (else
              (`Actor.K2_SetActorLocation` (`self.Marker`) (10000.0 10000.0 10000.0) false true))))))))

(event `Recharge`
  (`KismetSystemLibrary.Delay` (`self.RechargeDuration`))
  (set `self.Recharging` false))

(event `DecreaseUnreliability`
  (params (dt :type "Float (double-precision)"))
  ;[1 1 1] decreasing unreliability
  (if (>= (`self.UnreliablePercentage`) 0.0)
    (bind _result (`/Engine/EditorBlueprintResources/StandardMacros.NegateFloat` (* (`self.AddReliabilityPerSecond`) dt))
      (:`  `
        (`self.AddUnreliablility` _result)))))

(fn `AddUnreliablility`
  (params (amount :type "Float (double-precision)"))
  (set `self.UnreliablePercentage` (+ amount (`self.UnreliablePercentage`))))

(fn `CalculateLandingPosition`
  (returns (LandingPosition :type "Vector Structure"))
  (return (+ (`KismetMathLibrary.VLerp` (* (`SceneComponent.GetForwardVector` (`/Game/Blueprints/Character/Player_BP.GunBarrel` (`self.OwnerReference`))) (`self.MinDistance`)) (* (`SceneComponent.GetForwardVector` (`/Game/Blueprints/Character/Player_BP.GunBarrel` (`self.OwnerReference`))) (`self.MaxDistance`)) (/ (`self.ChargeTimer`) (`self.MaxChargeTime`))) (`Actor.K2_GetActorLocation` (`self.OwnerReference`)))))