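; BP_Marker is a marker actor that highlights the BP_Tile beneath it.
; Each Tick it unhighlights the stored CurrentTile, then runs a long multi line trace on the Visibility channel, opposite the up vector of its Plane.
; The first hit actor that casts to BP_Tile is highlighted, stored as CurrentTile, and ends the search.
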(event `self.ReceiveTick`
  (params (DeltaSeconds :type "Float (single-precision)"))
  (bind _returnvalue (`self.K2_GetActorLocation`))
  (`|ExecutionSequence`
    (:`then_0`
      ;[1 1 1] Unhighlight the previous tile
      (`/Engine/EditorBlueprintResources/StandardMacros.IsValid` (`self.CurrentTile`)
        (:`Is Valid`
          (`/Game/Blueprints/Tiles/BP_Tile.Unhighlight` (`self.CurrentTile`)))))
    (:`then_1`
      ;[1 1 1] Check for tiles beneath the marker
      (bind _outhits (`KismetSystemLibrary.LineTraceMulti` _returnvalue (+ _returnvalue (* (`SceneComponent.GetUpVector` (`self.Plane`)) -10000.0)) "TraceTypeQuery1"))
      (for _array_element _outhits
        (bind _asbp_tile (cast `/Game/Blueprints/Tiles/BP_Tile` (`.HitActor` (`GameplayStatics.BreakHitResult` _array_element))))
        (`/Game/Blueprints/Tiles/BP_Tile.Highlight` _asbp_tile)
        (set `self.CurrentTile` _asbp_tile)
        (break)))))

(fn `UserConstructionScript`)