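; Game mode for Hot As Ice that sets up local players and drives dynamic fire/ice music from grid control.
; Init spawns and possesses a typed Player_BP per PlayerStart, adds the HUD and calls MainGame on the game instance.
; Tick compares BP_GridSystem type percentages, crossfading soundtracks when the dominant type changes.
; Both tracks fade out while the third type holds at least 90%; neutral soundtrack fades are unwired.
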(event `self.ReceiveBeginPlay`
  (`|ExecutionSequence`
    (:`then_0`
      (bind _outactors (`GameplayStatics.GetAllActorsOfClass` "/Game/Blueprints/Tiles/BP_GridSystem.BP_GridSystem_C"))
      (bind _output (`|GetArrayItem` _outactors))
      (`/Engine/EditorBlueprintResources/StandardMacros.IsValid` _output
        (:`Is Valid`
          (set `self.GridSystemRef` _output))))
    (:`then_1`
      (set `PlayerController.bShowMouseCursor` true (`GameplayStatics.GetPlayerController` 0)))))

(event `self.ReceiveTick`
  (params (DeltaSeconds :type "Float (single-precision)"))
  (if (>= (`/Game/Blueprints/Tiles/BP_GridSystem.GetPercentage` (`self.GridSystemRef`) "NewEnumerator2") 0.9)
    (`KismetSystemLibrary.PrintString` "Hello" true true (struct :`G` 0.66 :`B` 1.0 :`A` 1.0) 0.0)
    (`AudioComponent.FadeOut` (`self.SC_FireSoundtrack`) (`self.FadeOutDuration`) 0.0)
    (`AudioComponent.FadeOut` (`self.SC_IceSoundtrack`) (`self.FadeOutDuration`) 0.0)
    (elif (> (`/Game/Blueprints/Tiles/BP_GridSystem.GetPercentage` (`self.GridSystemRef`) "NewEnumerator0") (`/Game/Blueprints/Tiles/BP_GridSystem.GetPercentage` (`self.GridSystemRef`) "NewEnumerator1"))
      (if (`|EnumInequality` (`self.PrevDominator`) "NewEnumerator0")
        (set `self.PrevDominator` "NewEnumerator0")
        (`AudioComponent.FadeIn` (`self.SC_IceSoundtrack`) (`self.FadeInDuration`) (`self.VolumeLevel`) 0.0)
        (`AudioComponent.FadeOut` (`self.SC_FireSoundtrack`) (`self.FadeOutDuration`) 0.0))
      (elif (`|EnumInequality` (`self.PrevDominator`) "NewEnumerator1")
        (set `self.PrevDominator` "NewEnumerator1")
        (`AudioComponent.FadeIn` (`self.SC_FireSoundtrack`) (`self.FadeInDuration`) (`self.VolumeLevel`) 0.0)
        (`AudioComponent.FadeOut` (`self.SC_IceSoundtrack`) (`self.FadeOutDuration`) 0.0)))))

(fn `Init`
  (bind _outactors (`GameplayStatics.GetAllActorsOfClass` "/Script/Engine.PlayerStart"))
  (for (_array_element _array_index) _outactors
    (`GameplayStatics.CreatePlayer` _array_index)
    (bind _returnvalue (`|SpawnActorFromClass` "/Game/Blueprints/Character/Player_BP.Player_BP_C" (`SceneComponent.K2_GetComponentToWorld` (`Actor.RootComponent` _array_element)) "Undefined" "OverrideRootScale" null null))
    (`Controller.Possess` (`GameplayStatics.GetPlayerController` _array_index) _returnvalue)
    (set `/Game/Blueprints/Character/Player_BP.Index` _array_index _returnvalue)
    (if (== _array_index 0)
      (set `/Game/Blueprints/Character/Player_BP.Type` "NewEnumerator1" _returnvalue)
      (else
        (set `/Game/Blueprints/Character/Player_BP.Type` "NewEnumerator0" _returnvalue)))
    (`/Game/Blueprints/Character/BP_Health.Init` (`/Game/Blueprints/Character/Player_BP.BP_Health` _returnvalue)))
  (bind _returnvalue_2 (`|CreateWidget` "/Game/Blueprints/UI/UI_HUD_BP.UI_HUD_BP_C"))
  (bind _output_get (set `self.UI` _returnvalue_2))
  (`UserWidget.AddToViewport` _returnvalue_2 0)
  (`UserWidget.AddToViewport` _output_get 0)
  (bind _asgi_hot_as_ice (cast `/Game/Blueprints/GameMode/GI_HotAsIce` (`GameplayStatics.GetGameInstance`)))
  (`/Game/Blueprints/GameMode/GI_HotAsIce.MainGame` _asgi_hot_as_ice))

(fn `UserConstructionScript`)