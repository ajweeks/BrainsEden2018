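; Game instance for Hot As Ice that runs a two-player match, keeping scores and pause state across level reloads.
; A death credits the other player, reloads the level and disables both players' inputs.
; The first to three wins ends the match; otherwise a timer calls UnpauseGame, which re-enables player one but leaves player two's DisableInputs true.
; Helpers expose the countdown and winner text.
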(event `MainGame`
  (set `self.IsPaused` true)
  (set `self.IsStartGame` false))

(event `StartGame`
  (set `self.PauseTimer` (struct))
  (set `self.IsPaused` false)
  (set `self.IsStartGame` true)
  (set `self.Player2_Wins` 0)
  (set `self.Player1_Wins` 0)
  (set `self.IsEndGame` false)
  (bind _asplayer_bp (cast `/Game/Blueprints/Character/Player_BP` (`Controller.K2_GetPawn` (`GameplayStatics.GetPlayerController` 0))))
  (set `/Game/Blueprints/Character/Player_BP.DisableInputs` false _asplayer_bp)
  (bind _asplayer_bp_2 (cast `/Game/Blueprints/Character/Player_BP` (`Controller.K2_GetPawn` (`GameplayStatics.GetPlayerController` 1))))
  (set `/Game/Blueprints/Character/Player_BP.DisableInputs` false _asplayer_bp_2))

(event `ExitGame`
  (`KismetSystemLibrary.QuitGame` null "Quit"))

(event `PlayerWinAndChecks`
  (params (playerID :type Integer))
  (if (`self.IsEndGame`)
    (set `self.IsStartGame` false :!label _label)
    (set `self.IsPaused` true)
    (set `self.IsEndGame` true)
    (else
      (`self.PlayerWin` playerID)
      (bind _win (`self.WinGame`))
      (if _win
        (bind _returnvalue (`GameplayStatics.GetCurrentLevelName` true))
        (`GameplayStatics.OpenLevel` (`KismetStringLibrary.Conv_StringToName` _returnvalue))
        (`KismetSystemLibrary.Delay` 0.15)
        (bind _asplayer_bp (cast `/Game/Blueprints/Character/Player_BP` (`Controller.K2_GetPawn` (`GameplayStatics.GetPlayerController` 0))))
        (set `/Game/Blueprints/Character/Player_BP.DisableInputs` true _asplayer_bp)
        (bind _asplayer_bp_2 (cast `/Game/Blueprints/Character/Player_BP` (`Controller.K2_GetPawn` (`GameplayStatics.GetPlayerController` 1))))
        (set `/Game/Blueprints/Character/Player_BP.DisableInputs` true _asplayer_bp_2)
        (goto _label)
        (else
          (bind _returnvalue_2 (`GameplayStatics.GetCurrentLevelName` true))
          (`GameplayStatics.OpenLevel` (`KismetStringLibrary.Conv_StringToName` _returnvalue_2))
          (set `self.IsPaused` true)
          (bind _returnvalue_3 (`KismetSystemLibrary.K2_SetTimer` null "UnpauseGame" 3.0))
          (set `self.PauseTimer` _returnvalue_3)
          (`KismetSystemLibrary.Delay` 0.15)
          (bind _asplayer_bp_3 (cast `/Game/Blueprints/Character/Player_BP` (`Controller.K2_GetPawn` (`GameplayStatics.GetPlayerController` 0))))
          (set `/Game/Blueprints/Character/Player_BP.DisableInputs` true _asplayer_bp_3)
          (bind _asplayer_bp_4 (cast `/Game/Blueprints/Character/Player_BP` (`Controller.K2_GetPawn` (`GameplayStatics.GetPlayerController` 1))))
          (set `/Game/Blueprints/Character/Player_BP.DisableInputs` true _asplayer_bp_4))))))

(fn `GetPausedTimeLeft`
  (returns (remainingTime :type "Float (double-precision)"))
  (return (`KismetSystemLibrary.K2_GetTimerRemainingTimeHandle` (`self.PauseTimer`))))

(fn `GetPlayerWon`
  (returns (Won :type String))
  (if (>= (`self.Player1_Wins`) 3)
    (return "Player one won!!!")
    (else
      (return "Player two won!!!"))))

(fn `PlayerWin`
  (params (DeathPlayer :type Integer))
  (if (`self.IsEndGame`)
    _
    (elif (== DeathPlayer 0)
      (bind _result (`/Engine/EditorBlueprintResources/StandardMacros.IncrementInt` (`self.Player2_Wins`))
        (:`  `
          (set `self.Player2_Wins` _result)))
      (else
        (bind _result_2 (`/Engine/EditorBlueprintResources/StandardMacros.IncrementInt` (`self.Player1_Wins`))
          (:`  `
            (set `self.Player1_Wins` _result_2)))))))

(fn `UnpauseGame`
  (`GameplayStatics.SetGamePaused` false)
  (set `self.IsPaused` false)
  (bind _asplayer_bp (cast `/Game/Blueprints/Character/Player_BP` (`Controller.K2_GetPawn` (`GameplayStatics.GetPlayerController` 0))))
  (set `/Game/Blueprints/Character/Player_BP.DisableInputs` false _asplayer_bp)
  (bind _asplayer_bp_2 (cast `/Game/Blueprints/Character/Player_BP` (`Controller.K2_GetPawn` (`GameplayStatics.GetPlayerController` 1))))
  (set `/Game/Blueprints/Character/Player_BP.DisableInputs` true _asplayer_bp_2))

(fn `WinGame`
  (returns (WIn :type Boolean) (WinnerID :type Integer))
  (if (>= (`self.Player1_Wins`) 3)
    (return true 0)
    (elif (>= (`self.Player2_Wins`) 3)
      (return true 1)
      (else
        (return false 0)))))