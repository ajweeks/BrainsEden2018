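; Player-fired projectile for a two-player game, appearing as an icicle or meteor based on the owner's Ice or Fire type.
; It lerps from begin to end point over its travel time, adding an accumulating pull toward the opponent within an auto-aim cone and radius.
; Opponent hits deal damage, knockback and rumble.
; Hits or timeout recolor tiles beneath; these and wall hits recharge the owner's weapon and explode the projectile.
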(event `self.ReceiveBeginPlay`
  (`KismetSystemLibrary.Delay` 0.0)
  (`|ExecutionSequence`
    (:`then_0`
      (bind _asplayer_bp (cast `/Game/Blueprints/Character/Player_BP` (`self.GetOwner`)))
      (bind _outactors (`GameplayStatics.GetAllActorsOfClass` "/Game/Blueprints/Character/Player_BP.Player_BP_C"))
      (bind _output (`|GetArrayItem` _outactors))
      (if (== _output _asplayer_bp)
        (set `self.Opponent` (`|GetArrayItem` _outactors 1))
        (else
          (set `self.Opponent` _output)))
      (switch `/Game/Blueprints/Character/Types` (`/Game/Blueprints/Character/Player_BP.Type` _asplayer_bp)
        (:`NewEnumerator0`
          (`StaticMeshComponent.SetStaticMesh` (`self.ProjectileMesh`) "/Game/Art_Assets/ME_Icycle_One.ME_Icycle_One")
          (`SceneComponent.K2_AddLocalRotation` (`self.ProjectileMesh`) (struct :`Roll` 90.0) false true)
          (`GameplayStatics.SpawnEmitterAttached` "/Game/Particles/P_Icycle.P_Icycle" (`self.Root`) "None" (0.0 0.0 0.0) (struct :`Roll` 90.0)))
        (:`NewEnumerator1`
          (`StaticMeshComponent.SetStaticMesh` (`self.ProjectileMesh`) "/Game/Art_Assets/ME_Meteor_One.ME_Meteor_One")
          (`SceneComponent.K2_AddLocalRotation` (`self.ProjectileMesh`) (`KismetMathLibrary.RandomRotator` true) false true)
          (`GameplayStatics.SpawnEmitterAttached` "/Game/Particles/P_Fireball.P_Fireball" (`self.Root`) "None" (0.0 0.0 0.0) (struct :`Roll` 90.0)))))
    (:`then_1`
      (set `self.Velocity` (`self.GetActorForwardVector`)))))

(event `self.ReceiveTick`
  (params (DeltaSeconds :type "Float (single-precision)"))
  (bind _returnvalue (`self.K2_GetActorLocation`))
  (bind _opponent (`self.Opponent`))
  (bind _autoaimradius (`self.AutoAimRadius`))
  (bind _returnvalue_2 (- (`self.K2_GetActorLocation` _opponent) (`self.K2_GetActorLocation`)))
  (bind _returnvalue_3 (`KismetMathLibrary.VSize` _returnvalue_2))
  (bind _returnvalue_4 (+ (`KismetMathLibrary.VLerp` (`self.BeginPoint`) (`self.EndPoint`) (/ (`self.TravelTimer`) (`self.TravelTime`))) (`self.PlayerPullOffset`)))
  (bind _returnvalue_5 (`KismetMathLibrary.Dot_VectorVector` (`KismetMathLibrary.Normal` (`self.Velocity`)) (`KismetMathLibrary.Normal` _returnvalue_2)))
  (`|ExecutionSequence`
    (:`then_0`
      (set `self.TravelTimer` (+ (`self.TravelTimer`) (`GameplayStatics.GetWorldDeltaSeconds`))))
    (:`then_1`
      (if (`KismetSystemLibrary.IsValid` _opponent)
        (`KismetSystemLibrary.PrintString` (`KismetStringLibrary.Conv_DoubleToString` _returnvalue_5))
        (if (and (> _returnvalue_5 (`self.AutoAimConeAngle`)) (<= _returnvalue_3 _autoaimradius))
          (bind _output_get (set `self.PlayerPullOffset` (+ (`self.PlayerPullOffset`) (* _returnvalue_2 (* DeltaSeconds (`self.AutoAimStrength`) (- 1.0 (`KismetMathLibrary.FClamp` (/ _returnvalue_3 _autoaimradius))))))))
          (`KismetSystemLibrary.PrintString` (`KismetStringLibrary.Conv_VectorToString` _output_get) false))))
    (:`then_2`
      (set `self.Velocity` (- _returnvalue_4 (`self.K2_GetActorLocation`)))
      (`self.K2_SetActorLocation` _returnvalue_4 true))
    (:`then_3`
      ;[1 1 1] Destroy the projectile
      (if (>= (`self.TravelTimer`) (`self.TravelTime`))
        (`|ExecutionSequence` :!label _label
          (:`then_0`
            ;[1 1 1] Color the tile beneath
            (bind _outhits (`KismetSystemLibrary.LineTraceMultiForObjects` _returnvalue (+ _returnvalue (* (`SceneComponent.GetUpVector` (`self.Root`)) -1000.0)) (`|MakeArray` "ObjectTypeQuery1" :!type "EObjectTypeQuery Enum")))
            (for _array_element _outhits
              (bind _asbp_tile (cast `/Game/Blueprints/Tiles/BP_Tile` (`.HitActor` (`GameplayStatics.BreakHitResult` _array_element))))
              (bind _asplayer_bp (cast `/Game/Blueprints/Character/Player_BP` (`self.GetOwner`)))
              (switch `/Game/Blueprints/Character/Types` (`/Game/Blueprints/Character/Player_BP.Type` _asplayer_bp)
                (:`NewEnumerator0`
                  (set `/Game/Blueprints/Tiles/BP_Tile.FrozenAmount` 0.0 _asbp_tile)
                  (break))
                (:`NewEnumerator1`
                  (set `/Game/Blueprints/Tiles/BP_Tile.FrozenAmount` 2.0 _asbp_tile)
                  (break)))))
          (:`then_1`
            (bind _asplayer_bp_2 (cast `/Game/Blueprints/Character/Player_BP` (`self.GetOwner`) :!label _label_2))
            (bind _bp_weapon (`/Game/Blueprints/Character/Player_BP.BP_Weapon` _asplayer_bp_2))
            (set `/Game/Blueprints/Character/BP_Weapon.FireballRef` null _bp_weapon)
            (`/Game/Blueprints/Character/BP_Weapon.Recharge` _bp_weapon)
            (`GameplayStatics.PlaySound2D` "/Game/Sound/SC_HittingWall.SC_HittingWall")
            (bind _asplayer_bp_3 (cast `/Game/Blueprints/Character/Player_BP` (`self.GetOwner`)))
            (switch `/Game/Blueprints/Character/Types` (`/Game/Blueprints/Character/Player_BP.Type` _asplayer_bp_3)
              (:`NewEnumerator0`
                (`GameplayStatics.SpawnEmitterAtLocation` "/Game/Particles/P_IcycleExplosion.P_IcycleExplosion" (`self.K2_GetActorLocation`)))
              (:`NewEnumerator1`
                (`GameplayStatics.SpawnEmitterAtLocation` "/Game/Particles/P_FireballExplosion.P_FireballExplosion" (`self.K2_GetActorLocation`))))
            (`self.K2_DestroyActor`)))))))

(event `self.ProjectileMesh.OnComponentBeginOverlap`
  (params (OverlappedComponent :type "PrimitiveComponent Object Reference") (OtherActor :type "Actor Object Reference") (OtherComp :type "PrimitiveComponent Object Reference") (OtherBodyIndex :type Integer) (bFromSweep :type Boolean) (SweepResult :type "HitResult Structure (by ref)"))
  (bind _asplayer_bp (cast `/Game/Blueprints/Character/Player_BP` OtherActor)
    (:`then`
      (if (!= _asplayer_bp (`self.GetOwner`))
        (`/Game/Blueprints/Character/BP_Health.TakeDamageAndCheck` (`/Game/Blueprints/Character/Player_BP.BP_Health` _asplayer_bp) (`self.ProjectileDamage`) (0.0 0.0 0.0))
        (`|ExecutionSequence`
          (:`then_0`
            (`PlayerController.PlayDynamicForceFeedback` (`GameplayStatics.GetPlayerController` (`/Game/Blueprints/Character/Player_BP.Index` _asplayer_bp)) 1.0 0.25 true true true true))
          (:`then_1`
            (set `/Game/Blueprints/Character/Player_BP.Hurt` false _asplayer_bp)
            (`GameplayStatics.PlaySound2D` "/Game/Sound/SC_HittingPlayer.SC_HittingPlayer")
            (bind (_returnvalue_x _returnvalue_y) (`KismetMathLibrary.BreakVector` (* (`KismetMathLibrary.Normal` (- (`self.K2_GetActorLocation` _asplayer_bp) (`self.K2_GetActorLocation`))) 1000.0)))
            (`Character.LaunchCharacter` _asplayer_bp (`KismetMathLibrary.MakeVector` _returnvalue_x _returnvalue_y 10.0) true false)
            (`KismetSystemLibrary.PrintString` "LAUNCH CHARACTER")
            (goto _label)))))
    (:`CastFailed`
      (if (`self.ActorHasTag` OtherActor "Wall")
        (goto _label_2)))))

(event `Custom Destroy`
  (goto _label_2))

(fn `UserConstructionScript`
  (`SceneComponent.SetWorldScale3D` (`self.ProjectileMesh`) (0.3 0.3 0.3)))