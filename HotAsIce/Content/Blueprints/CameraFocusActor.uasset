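; CameraFocusActor is a shared camera for two players that follows their midpoint and zooms with their separation.
; On BeginPlay it initializes the game mode, becomes the player controllers' view target, and registers itself with both Player_BP actors before initializing them.
; Each Tick it centers between them, sets clamped spring arm length from their distance, and applies a decaying shake offset.
; AddShake replaces that offset rather than accumulating it.
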(event `self.ReceiveBeginPlay`
  (bind _asbase_game_mode (cast `/Game/Blueprints/GameMode/BaseGameMode` (`GameplayStatics.GetGameMode`)))
  (`/Game/Blueprints/GameMode/BaseGameMode.Init` _asbase_game_mode)
  (bind _outactors (`GameplayStatics.GetAllActorsOfClass` "/Script/Engine.PlayerController"))
  (`PlayerController.SetViewTargetWithBlend` _outactors self 0.0 "VTBlend_Linear" 0.0 false)
  (bind _outactors_2 (`GameplayStatics.GetAllActorsOfClass` "/Game/Blueprints/Character/Player_BP.Player_BP_C"))
  (bind _output_get (set `self.Player0` (`|GetArrayItem` _outactors_2)))
  (set `/Game/Blueprints/Character/Player_BP.Camera` self _output_get)
  (`/Game/Blueprints/Character/Player_BP.Init` _output_get)
  (bind _output_get_2 (set `self.Player1` (`|GetArrayItem` _outactors_2 1)))
  (set `/Game/Blueprints/Character/Player_BP.Camera` self _output_get_2)
  (`/Game/Blueprints/Character/Player_BP.Init` _output_get_2))

(event `self.ReceiveTick`
  (params (DeltaSeconds :type "Float (single-precision)"))
  (bind _playerdisplacement (`self.PlayerDisplacement`))
  (`|ExecutionSequence`
    (:`then_0`
      (set `self.PlayerDisplacement` (- (`self.K2_GetActorLocation` (`self.Player0`)) (`self.K2_GetActorLocation` (`self.Player1`))))
      (`self.K2_SetActorLocation` (+ (`self.K2_GetActorLocation` (`self.Player1`)) (/ _playerdisplacement 2.0) (`self.Shake`)))
      (set `SpringArmComponent.TargetArmLength` (`KismetMathLibrary.FClamp` (`KismetMathLibrary.VSize` _playerdisplacement) (`self.MinArmLength`) (`self.MaxArmLength`)) (`self.SpringArm`)))
    (:`then_1`
      (set `self.Shake` (* (`self.Shake`) (`self.ShakeDecay`))))))

(fn `AddShake`
  (params (Shake :type "Vector Structure"))
  (set `self.Shake` Shake))

(fn `UserConstructionScript`)