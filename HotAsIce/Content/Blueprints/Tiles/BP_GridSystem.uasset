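; BP_GridSystem is a grid actor that spawns a two-dimensional field of BP_Tile actors when play begins.
; SpawnGrid runs nested row and column loops bounded by GridSize, offsetting each tile from the actor's location by TileSize along X and Y.
; Tiles always spawn regardless of collision and are stored in a Tiles array, whose length GetTileCount returns.
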(event `self.ReceiveBeginPlay`
  (`self.SpawnGrid`))

(fn `GetTileCount`
  (returns (TileCount :type Integer))
  (return (`KismetArrayLibrary.Array_Length` (`self.Tiles`))))

(fn `SpawnGrid`
  (locals (Row :type Integer) (Column :type Integer))
  (bind _gridsize_x (`KismetMathLibrary.BreakVector2D` (`self.GridSize`)))
  (bind (_gridsize_x_2 _gridsize_y) (`KismetMathLibrary.BreakVector2D` (`self.GridSize`)))
  (for _index (range (+ (`KismetMathLibrary.FTrunc` _gridsize_x) 1))
    (set `local.Row` _index)
    (for _index_2 (range (+ (`KismetMathLibrary.FTrunc` _gridsize_y) 1))
      (set `local.Column` _index_2)
      (bind _returnvalue (`|SpawnActorFromClass` "/Game/Blueprints/Tiles/BP_Tile.BP_Tile_C" (`KismetMathLibrary.MakeTransform` (+ (`self.K2_GetActorLocation`) (`KismetMathLibrary.MakeVector` (* (`local.Row`) (`self.TileSize`)) (* (`local.Column`) (`self.TileSize`))))) "AlwaysSpawn" "OverrideRootScale" null null))
      (`KismetArrayLibrary.Array_Add` (`self.Tiles`) _returnvalue))))

(fn `UserConstructionScript`)