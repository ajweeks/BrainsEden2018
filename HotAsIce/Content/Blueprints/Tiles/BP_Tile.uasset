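; Tile actor that tracks a FrozenAmount, shows it through a dynamic material and derives one of three tile types from it.
; Each Tick clamps the amount, writes it to the material, drifts it back toward the neutral midpoint via Decay, then reclassifies Type by thresholds.
; A type change fires ChangeTypePolish, an empty hook.
; Cooldown lowers the amount over time but is not called here.
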(event `self.ReceiveTick`
  (params (DeltaSeconds :type "Float (single-precision)"))
  (`|ExecutionSequence`
    (:`then_0`
      (if (< (`self.FrozenAmount`) 0.0)
        (set `self.FrozenAmount` 0.0)))
    (:`then_1`
      (if (> (`self.FrozenAmount`) 2.0)
        (set `self.FrozenAmount` 2.0)))
    (:`then_2`
      (`MaterialInstanceDynamic.SetScalarParameterValue` (`self.TileMaterial`) "Enum" (`self.FrozenAmount`))
      (`self.Decay`))
    (:`then_3`
      (bind _foundtype (`self.CheckType`))
      (if (!= _foundtype (`self.Type`))
        (`self.ChangeTypePolish`))
      (set `self.Type` _foundtype))))

(event `ChangeTypePolish`)

(fn `CheckType`
  (returns (FoundType :type "/Game/Blueprints/Character/Types Enum"))
  (`|ExecutionSequence`
    (:`then_0`
      (if (<= (`self.FrozenAmount`) 0.5)
        (return "NewEnumerator0")))
    (:`then_1`
      (if (>= (`self.FrozenAmount`) 1.5)
        (return "NewEnumerator1")))
    (:`then_2`
      (return "NewEnumerator2"))))

(fn `Cooldown`
  (params (Amount :type "Float (double-precision)"))
  (set `self.FrozenAmount` (- (`self.FrozenAmount`) (* (`GameplayStatics.GetWorldDeltaSeconds`) Amount))))

(fn `Decay`
  (`|ExecutionSequence`
    (:`then_0`
      (if (<= (`self.FrozenAmount`) 1.0)
        (set `self.FrozenAmount` (+ (`self.FrozenAmount`) (* (`GameplayStatics.GetWorldDeltaSeconds`) (`self.DecayAmount`))))))
    (:`then_1`
      (if (>= (`self.FrozenAmount`) 1.0)
        (set `self.FrozenAmount` (- (`self.FrozenAmount`) (* (`GameplayStatics.GetWorldDeltaSeconds`) (`self.DecayAmount`))))))))

(fn `UserConstructionScript`
  (bind _returnvalue (`PrimitiveComponent.CreateDynamicMaterialInstance` (`self.Cube`) 0 "/Game/Materials/Tiles/M_Tile.M_Tile"))
  (set `self.TileMaterial` _returnvalue))